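; RocketBP is a rocket hazard that plays a missile warning, hides its mesh after a delay, then plays an explosion sound and destroys itself.
; A collision overlap with a tagged Player in mech form spawns an explosion and destroys the rocket.
; Otherwise it kills the player: ragdolls the mesh, stops movement, switches to UI input and fades in the HUD death screen through a timeline.
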(event `self.ReceiveBeginPlay`
  (`GameplayStatics.PlaySound2D` "/Game/Sounds/missile_warning.missile_warning" 1.0 1.0 0.0 null null)
  (`KismetSystemLibrary.Delay` 3.0)
  (`SceneComponent.SetVisibility` (`self.StaticMesh`) false false)
  (`KismetSystemLibrary.Delay` 2.0)
  (`GameplayStatics.PlaySound2D` "/Game/Sounds/rocket_explode_1.rocket_explode_1" 1.0 1.0 0.0 null null)
  (`self.K2_DestroyActor`))

(event `self.Collision.OnComponentBeginOverlap`
  (params (OverlappedComponent :type "PrimitiveComponent Object Reference") (OtherActor :type "Actor Object Reference") (OtherComp :type "PrimitiveComponent Object Reference") (OtherBodyIndex :type Integer) (bFromSweep :type Boolean) (SweepResult :type "HitResult Structure (by ref)"))
  (bind _returnvalue (`GameplayStatics.GetPlayerController` 0))
  (if (`self.ActorHasTag` OtherActor "Player")
    (bind _asplayer (cast `/Game/Player` OtherActor))
    (if (`/Game/Player.IsMech` _asplayer)
      (`GameplayStatics.PlaySound2D` "/Game/Sounds/Explosion01.Explosion01" 1.0 1.0 0.0 null null)
      (`GameplayStatics.SpawnEmitterAtLocation` "/Game/VFX/ParticleMats/P_Explosion.P_Explosion" (`self.K2_GetActorLocation`))
      (`self.K2_DestroyActor`)
      (else
        (`PrimitiveComponent.SetSimulatePhysics` (`Character.Mesh` _asplayer) true)
        (set `/Game/Player.MovementSpeed` 0.0 _asplayer)
        (set `/Game/Player.Alive?` false _asplayer)
        (`WidgetBlueprintLibrary.SetInputMode_UIOnlyEx` _returnvalue null)
        (set `PlayerController.bShowMouseCursor` true _returnvalue)
        (bind (_direction _death) (`Timeline|Timeline` :!via `PlayFromStart`)
          (:`Update`
            (`Widget.SetRenderOpacity` (`/Game/HUD.DeathScreen` (`/Game/Player.Hud` _asplayer)) _death)
            (`/Engine/EditorBlueprintResources/StandardMacros.DoOnce` false
              (:`Completed`
                (`GameplayStatics.PlaySound2D` "/Game/DeathSound.DeathSound" 1.0 1.0 0.0 null null))))
          (:`Finished`
            (`self.K2_DestroyActor`)))))))

(fn `UserConstructionScript`)